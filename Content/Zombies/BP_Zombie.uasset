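; Zombie enemy that chases the player, attacks in melee and reports its death to the game mode.
; It spawns with a random skin and attached sound, then loops AI MoveTo into an attack montage, retrying on failure.
; RightHand overlaps damage the first-person character.
; Regular and radial damage share a one-shot death path that notifies the game mode, ragdolls the mesh, disables collision, stops the sound and destroys the actor after a delay.
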(event OnComponentBeginOverlap(RightHand)
  (params (OverlappedComponent :type Primitive%20Component%20Object%20Reference) (OtherActor :type Actor%20Object%20Reference) (OtherComp :type Primitive%20Component%20Object%20Reference) (OtherBodyIndex :type Integer) (bFromSweep :type Boolean) (SweepResult :type Hit%20Result%20Structure%20%28by%20ref%29))
  (bind _asbp_first_person_character (Utilities|Casting|CastToBP_FirstPersonCharacter OtherActor))
  (Game|Damage|ApplyDamage _asbp_first_person_character 1e+01 0 0)
  (Development|PrintString (Utilities|GetDisplayName self)))

(event Custom|ChasePlayer
  (Variables|Default|SetisRunning true)
  (AI|AIMoveTo self "0, 0, 0" (Game|GetPlayerController 0) 1e+02 false
    (:OnSuccess
      (Animation|Montage|PlayMontage (Variables|Character|GetMesh) "/Game/Zombies/AS_Zombie_Attack_Montage.AS_Zombie_Attack_Montage" 1.6
        (:then
          (Variables|Default|SetisRunning false))
        (:OnCompleted
          (CallFunction|ChasePlayer))))
    (:OnFail
      (CallFunction|ChasePlayer))))

(event EventBeginPlay
  (Components|SkeletalMesh|SetSkeletalMeshAsset (Variables|Character|GetMesh) (.OutItem (Utilities|Array|Random (Variables|Default|GetSkins))))
  (CallFunction|ChasePlayer)
  (bind _returnvalue (Audio|SpawnSoundAttached "/Game/Zombies/zombie-throat-filled-with-liquid.zombie-throat-filled-with-liquid" (Variables|Character|GetMesh) "None" "0, 0, 0" "0, 0, 0" "KeepRelativeOffset" true 0.1 1.0 0.0 "/Game/Weapons_And_Items/Bomb_-_C4/SA_BombTicking.SA_BombTicking" 0)))

(event Game|Damage|EventAnyDamage
  (params (Damage :type Float%20%28single-precision%29) (DamageType :type Damage%20Type%20Object%20Reference) (InstigatedBy :type Controller%20Object%20Reference) (DamageCauser :type Actor%20Object%20Reference))
  (bind _output_get (Variables|Default|SetHealth (- (Variables|Default|GetHealth) Damage)))
  (if (<= _output_get 0.0)
    (Utilities|FlowControl|DoOnce false
      (:Completed
        (bind _asbp_zombie_game_mod (Utilities|Casting|CastToBp_ZombieGameMod (Game|GetGameMode)))
        (Default|ZombieDying _asbp_zombie_game_mod)
        (Physics|SetSimulatePhysics (Variables|Character|GetMesh) true)
        (Collision|SetCollisionEnabled (Variables|Collision|GetCapsuleComponent) "NoCollision")
        (Utilities|IsValid (stale EventBeginPlay _returnvalue)
          (:Is%20Valid
            (Audio|Components|Audio|Stop (stale EventBeginPlay _returnvalue)))
          (:Is%20Not%20Valid
            _))
        (Utilities|FlowControl|Delay 5.0)
        (Actor|DestroyActor)))))

(event Game|Damage|EventRadialDamage
  (params (DamageReceived :type Float%20%28single-precision%29) (DamageType :type Damage%20Type%20Object%20Reference) (Origin :type Vector :default "0, 0, 0") (HitInfo :type Hit%20Result%20Structure%20%28by%20ref%29) (InstigatedBy :type Controller%20Object%20Reference) (DamageCauser :type Actor%20Object%20Reference))
  (bind _output_get (Variables|Default|SetHealth (- (Variables|Default|GetHealth) DamageReceived)))
  (if (<= _output_get 0.0)
    (Utilities|FlowControl|DoOnce false
      (:Completed
        (bind _asbp_zombie_game_mod (Utilities|Casting|CastToBp_ZombieGameMod (Game|GetGameMode)))
        (Default|ZombieDying _asbp_zombie_game_mod)
        (Physics|SetSimulatePhysics (Variables|Character|GetMesh) true)
        (Collision|SetCollisionEnabled (Variables|Collision|GetCapsuleComponent) "NoCollision")
        (Utilities|IsValid (stale EventBeginPlay _returnvalue)
          (:Is%20Valid
            (Audio|Components|Audio|Stop (stale EventBeginPlay _returnvalue)))
          (:Is%20Not%20Valid
            _))
        (Utilities|FlowControl|Delay 5.0)
        (Actor|DestroyActor)))))

(fn ConstructionScript)